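; BP_Dagger is a dagger that a motion controller can pick up and drop, and that knocks back enemies it touches.
; Pickup disables physics and snaps it to the hand mesh at a fixed offset, while Drop detaches it and restores physics.
; Static mesh overlaps with EnemyTestBP launch that character horizontally away with added lift, scaled by LaunchVelocity.
; The construction script assigns Box as Weapon's collision mesh for testing.
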(event `self.ReceiveBeginPlay`)

(event `/Game/VirtualRealityBP/Blueprints/PickupActorInterface.Pickup`
  (params (MotionController :type "SceneComponent Object Reference") (HandMesh :type "SceneComponent Object Reference"))
  (`PrimitiveComponent.SetSimulatePhysics` (`self.StaticMeshComponent`) false)
  (`SceneComponent.K2_AttachToComponent` (`self.K2_GetRootComponent`) HandMesh "None" "SnapToTarget" "SnapToTarget" "KeepWorld" false)
  (`SceneComponent.K2_SetRelativeLocationAndRotation` (`self.StaticMeshComponent`) (8.210977 -12.785643 -1.971997) (struct :`Roll` 90.0) false false))

(event `/Game/VirtualRealityBP/Blueprints/PickupActorInterface.Drop`
  (params (MotionController :type "SceneComponent Object Reference") (HandMesh :type "SceneComponent Object Reference"))
  (`PrimitiveComponent.SetSimulatePhysics` (`self.StaticMeshComponent`) true)
  (`self.K2_DetachFromActor` "KeepWorld" "KeepWorld" "KeepWorld"))

(event `Knockback`
  (params (Enemy :type "Character Object Reference"))
  (bind (_returnvalue_x _returnvalue_y) (`KismetMathLibrary.BreakVector` (`KismetMathLibrary.GetDirectionUnitVector` (`SceneComponent.K2_GetComponentLocation` (`self.StaticMeshComponent`)) (`self.K2_GetActorLocation` Enemy))))
  (bind (_returnvalue_x_2 _returnvalue_y_2) (`KismetMathLibrary.BreakVector` (`KismetMathLibrary.Normal` (`KismetMathLibrary.MakeVector` _returnvalue_x _returnvalue_y))))
  ;[1 1 1] Knockback The Player (Parameter will be whatever collided with the Attack Box)
  (`Character.LaunchCharacter` Enemy (* (`KismetMathLibrary.MakeVector` _returnvalue_x_2 _returnvalue_y_2 0.5) (`self.Launch Velocity`)) false false))

(event `self.StaticMeshComponent.OnComponentBeginOverlap`
  (params (OverlappedComponent :type "PrimitiveComponent Object Reference") (OtherActor :type "Actor Object Reference") (OtherComp :type "PrimitiveComponent Object Reference") (OtherBodyIndex :type Integer) (bFromSweep :type Boolean) (SweepResult :type "HitResult Structure (by ref)"))
  (bind _asenemy_test_bp (cast `/Game/Enemy/EnemyTestBP` OtherActor))
  (`self.Knockback` _asenemy_test_bp))

(fn `UserConstructionScript`
  ;[1 1 1] Testing Purposes
  (set `Weapon.CollisionMesh` (`self.Box`) (`self.Weapon`)))