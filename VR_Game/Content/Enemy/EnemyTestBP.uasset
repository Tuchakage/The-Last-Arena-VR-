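; Test enemy Blueprint that targets the player's motion controller pawn, with a blockable melee attack.
; BeginPlay stores the player as EnemyTarget, and AttackBox overlaps cache any CanBlock-tagged actor as the player's weapon.
; DoAttack damages the player's Health component unless that weapon overlaps the box, in which case the enemy damages itself as temporary test code.
; Tick destroys the enemy once its health drops below one.
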(event `self.ReceiveBeginPlay`
  ;[1 1 1] Set the Enemy Target To The Player (Makes it so Enemy will chase the player
  (set `self.EnemyTarget` (`GameplayStatics.GetPlayerPawn` 0)))

(event `DoAttack`
  (bind _returnvalue (`GameplayStatics.GetPlayerPawn` 0))
  ;[1 1 1] If The Attack Box Of Enemy Is Overlapping With The Player When the Attack Task is called then call the Players Take Damage Function
  ;[1 1 1] When this Event is called and the Attack Box is still overlapping the Blockable Weapon, Block Attack
  (if (`PrimitiveComponent.IsOverlappingActor` (`self.AttackBox`) (`self.PlayersWeapon`))
    (`KismetSystemLibrary.PrintString` "Blocking")
    ;[0.3698 0 0.02204] DELETE LATER (ONLY FOR TESTING)
    (`HealthComponent.TakeDamage` (`self.Health`) 100.0)
    (elif (`PrimitiveComponent.IsOverlappingActor` (`self.AttackBox`) _returnvalue)
      (bind _asmotion_controller_pawn (cast `/Game/VirtualRealityBP/Blueprints/MotionControllerPawn` _returnvalue))
      (`HealthComponent.TakeDamage` (`/Game/VirtualRealityBP/Blueprints/MotionControllerPawn.Health` _asmotion_controller_pawn) 100.0)
      (`KismetSystemLibrary.PrintString` "Player Attacked"))))

(event `self.ReceiveTick`
  (params (DeltaSeconds :type "Float (single-precision)"))
  ;[1 1 1] If Health is less than 1 then destroy the actor
  (if (< (`HealthComponent.currentHealth` (`self.Health`)) 1.0)
    (`self.K2_DestroyActor`)))

(event `self.AttackBox.OnComponentBeginOverlap`
  (params (OverlappedComponent :type "PrimitiveComponent Object Reference") (OtherActor :type "Actor Object Reference") (OtherComp :type "PrimitiveComponent Object Reference") (OtherBodyIndex :type Integer) (bFromSweep :type Boolean) (SweepResult :type "HitResult Structure (by ref)"))
  ;[1 1 1] If the attack Box is attacking the weapon then that means the player is blocking
  (if (`self.ActorHasTag` OtherActor "CanBlock")
    (set `self.PlayersWeapon` OtherActor)))

(fn `UserConstructionScript`)