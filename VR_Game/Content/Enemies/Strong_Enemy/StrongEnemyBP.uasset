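; Strong enemy character that targets the VR player and reports its spawn and death to VR_GameMode's alive count.
; DoAttack, unless blocked, damages a player overlapping AttackBox and shows a hurt widget.
; Tick watches health, then clears IsAlive, stops movement and runs a one-time death sound and delayed destroy.
; AllowMovement resets the Blocked and BeenHit flags for the animation state machine; the movement stop on those flags is unwired.
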(event `self.ReceiveBeginPlay`
  ;[1 1 1] Set the Enemy Target To The Player (Makes it so Enemy will chase the player
  (bind _asvrcharacter (cast `/Game/VirtualRealityBP/Blueprints/VRCharacter` (`GameplayStatics.GetPlayerPawn` 0)))
  (set `self.EnemyTarget` _asvrcharacter)
  ;[1 1 1] When Enemy Spawns tell GameMode that another enemy has spawned
  (bind _asvr_game_mode (cast `/Game/General/VR_GameMode` (`GameplayStatics.GetGameMode`)))
  (`/Engine/EditorBlueprintResources/StandardMacros.IncrementInt` (`/Game/General/VR_GameMode.EnemyAlive` _asvr_game_mode)))

(event `self.ReceiveTick`
  (params (DeltaSeconds :type "Float (single-precision)"))
  ;[1 1 1] If Health is less than 1 then play the death animation and after 3 seconds destroy the actor and tell the GameMode BP that there is one less Enemy alive
  (if (< (`HealthComponent.currentHealth` (`self.Health`)) 1.0)
    (bind _asvr_game_mode (cast `/Game/General/VR_GameMode` (`GameplayStatics.GetGameMode`)))
    ;;[1 1 1] Plays The Death Animation
    (set `self.isAlive` false)
    (`MovementComponent.StopMovementImmediately` (`self.CharacterMovement`))
    (`/Engine/EditorBlueprintResources/StandardMacros.DoOnce` false
      (:`Completed`
        (`GameplayStatics.PlaySoundAtLocation` "/Game/Sound/EnemyDeathSFX.EnemyDeathSFX" (`SceneComponent.K2_GetComponentLocation` (`self.Mesh`)) (struct) 1.0 1.0 0.0 null null null)
        (`KismetSystemLibrary.Delay` 3.0)
        (`/Engine/EditorBlueprintResources/StandardMacros.DecrementInt` (`/Game/General/VR_GameMode.EnemyAlive` _asvr_game_mode)
          (:`  `
            (`/Game/General/VR_GameMode.CheckEnemyLeft` _asvr_game_mode)
            (`self.K2_DestroyActor`)))))))

(event `DoAttack`
  (bind _returnvalue (`GameplayStatics.GetPlayerPawn` 0))
  ;[1 1 1] If the Enemy attack is not being blocked and If The Attack Box Of Enemy Is Overlapping With The Player When the Attack Task is called then call the Players Take Damage Function and adds a temporary red splash screen to the players UI
  (if (`self.Blocked`)
    _
    (elif (`PrimitiveComponent.IsOverlappingActor` (`self.AttackBox`) _returnvalue)
      (bind _asvrcharacter (cast `/Game/VirtualRealityBP/Blueprints/VRCharacter` _returnvalue))
      (`HealthComponent.TakeDamage` (`/Game/VirtualRealityBP/Blueprints/VRCharacter.Health` _asvrcharacter) 20.0)
      (bind _returnvalue_2 (`|CreateWidget` "/Game/General/UI/HurtWidget.HurtWidget_C"))
      (`UserWidget.AddToViewport` _returnvalue_2 0)
      (`KismetSystemLibrary.PrintString` "Player Attacked"))))

(event `AllowMovement`
  ;[1 1 1] If The Block animation Or Been Hit animation is still playing then set the variables back to false so that the state machine can go back to its original state and so the Enemy can go back to moving
  (if (or (`self.Blocked`) (`self.BeenHit`))
    (set `self.BeenHit` false)
    (set `self.Blocked` false)))

(fn `UserConstructionScript`)