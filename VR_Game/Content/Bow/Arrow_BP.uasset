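; Bow arrow projectile that flags an EnemyTestBP it overlaps as hit, then destroys itself.
; Shoot sets projectile speed, activates movement and enables query collision on the Box, which the construction script also assigns as the Weapon's collision mesh.
; Overlap briefly pulses the enemy's BeenHit using delays before destruction.
; SetArrowPower stores launch strength for a flattened, slightly upward Knockback launch, but the overlap's Knockback call is disconnected.
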(event `Knockback`
  (params (Enemy :type "Character Object Reference"))
  (bind (_returnvalue_x _returnvalue_y) (`KismetMathLibrary.BreakVector` (`KismetMathLibrary.GetDirectionUnitVector` (`SceneComponent.K2_GetComponentLocation` (`self.StaticMeshComponent`)) (`self.K2_GetActorLocation` Enemy))))
  (bind (_returnvalue_x_2 _returnvalue_y_2) (`KismetMathLibrary.BreakVector` (`KismetMathLibrary.Normal` (`KismetMathLibrary.MakeVector` _returnvalue_x _returnvalue_y))))
  ;[1 1 1] Knockback The Player (Parameter will be whatever collided with the Attack Box)
  (`Character.LaunchCharacter` Enemy (* (`KismetMathLibrary.MakeVector` _returnvalue_x_2 _returnvalue_y_2 0.5) (`self.Launch Velocity`)) false false))

(event `Shoot`
  (params (Velocity :type "Float (double-precision)"))
  (bind _projectilemovement (`self.ProjectileMovement`))
  ;[1 1 1] Makes the Arrow move forward
  (bind _output_get (set `ProjectileMovementComponent.InitialSpeed` Velocity _projectilemovement))
  (set `ProjectileMovementComponent.MaxSpeed` _output_get _projectilemovement)
  (`ProjectileMovementComponent.SetVelocityInLocalSpace` _projectilemovement (`KismetMathLibrary.MakeVector` Velocity))
  ;[1 1 1] Enable The Projectile Movement Component So Arrow can move
  (`ActorComponent.SetActive` (`self.ProjectileMovement`) true false)
  ;[1 1 1] Make it able to collide with something
  (`PrimitiveComponent.SetCollisionEnabled` (`self.Box`) "QueryOnly"))

(event `SetArrowPower`
  (params (Velocity :type "Float (double-precision)"))
  ;[1 1 1] Knockback The Player (Parameter will be whatever collided with the Attack Box)
  ;;[1 1 1] Set The Knockback Of The Arrow
  (set `self.Launch Velocity` Velocity))

(event `self.Box.OnComponentBeginOverlap`
  (params (OverlappedComponent :type "PrimitiveComponent Object Reference") (OtherActor :type "Actor Object Reference") (OtherComp :type "PrimitiveComponent Object Reference") (OtherBodyIndex :type Integer) (bFromSweep :type Boolean) (SweepResult :type "HitResult Structure (by ref)"))
  ;[1 1 1] When it collides with an Enemy push the Enemy backwards and destroy the arrow
  (bind _asenemy_test_bp (cast `/Game/Enemy/EnemyTestBP` OtherActor))
  (set `/Game/Enemy/EnemyTestBP.BeenHit` true _asenemy_test_bp)
  (`KismetSystemLibrary.Delay` 0.2)
  (set `/Game/Enemy/EnemyTestBP.BeenHit` false _asenemy_test_bp)
  (`KismetSystemLibrary.Delay` 0.2)
  (`self.K2_DestroyActor`))

(fn `UserConstructionScript`
  (set `Weapon.CollisionMesh` (`self.Box`) (`self.Weapon`)))