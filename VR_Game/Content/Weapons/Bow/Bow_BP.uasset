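; Two-handed VR bow that a motion controller picks up, draws and fires.
; The first hand attaches the bow to a hand socket; a second hand overlapping the string spawns an arrow and enables Tick.
; Tick projects that hand onto the bow's forward axis, limiting string travel and measuring charge.
; Releasing it plays a snap-back timeline that launches the arrow near its end, with speed and knockback scaled by charge.
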(event `/Game/VirtualRealityBP/Blueprints/PickupActorInterface.Pickup`
  (params (MotionController :type "SceneComponent Object Reference") (HandMesh :type "SceneComponent Object Reference") (HandEnum :type "/Game/VirtualRealityBP/Blueprints/WhichHand Enum" :default "NewEnumerator0") (SkeletalMesh :type "SkeletalMeshComponent Object Reference"))
  ;[1 1 1] Set which socket the bow will be attached to
  (switch `/Game/VirtualRealityBP/Blueprints/WhichHand` HandEnum
    (:`NewEnumerator0`
      (set `self.WhichHand` "Bow_L"))
    (:`NewEnumerator1`
      (set `self.WhichHand` "Bow_R")))
  ;[1 1 1] Check if the First Hand is there at all
  (`self.FirstHand`
    (:`then`
      ;[1 1 1] Check if any of the Actors its colliding to is the Motion Controller
      (for _array_element (`PrimitiveComponent.GetOverlappingActors` (`self.StringCollision`) "/Script/Engine.Actor")
        ;[1 1 1] Set The Second Hand to the motion controller because that is what we want to Track
        (if (== _array_element (`ActorComponent.GetOwner` MotionController))
          (set `self.SecondHand` MotionController)
          (`self.SetActorTickEnabled` true)
          ;[1 1 1] Spawn The Arrow In and attach it to the string of the bow but then after set the location of the arrow so it is not inside the bow and string
          (bind _returnvalue (`|SpawnActorFromClass` "/Game/Weapons/Bow/Arrow_BP.Arrow_BP_C" (`KismetMathLibrary.MakeTransform` (0.0 0.0 0.0) (struct) (1.0 1.0 1.0)) "AlwaysSpawn" "OverrideRootScale" null null))
          (bind _output_get (set `self.Arrow` _returnvalue))
          (`self.K2_AttachToComponent` _output_get (`self.String`) "None" "SnapToTarget" "SnapToTarget" "KeepWorld" false)
          (`self.K2_SetActorRelativeLocation` _output_get (33.0 0.0 0.0) false false))))
    (:`else`
      (set `self.FirstHand` HandMesh)
      (`PrimitiveComponent.SetSimulatePhysics` (`self.StaticMeshComponent`) false)
      (`SceneComponent.K2_AttachToComponent` (`self.StaticMeshComponent`) SkeletalMesh (`self.WhichHand`) "SnapToTarget" "SnapToTarget" "KeepWorld" false))))

(event `/Game/VirtualRealityBP/Blueprints/PickupActorInterface.Drop`
  (params (MotionController :type "SceneComponent Object Reference") (HandMesh :type "SceneComponent Object Reference"))
  (`KismetSystemLibrary.PrintString` (`KismetSystemLibrary.GetDisplayName` MotionController))
  ;[1 1 1] If Second Hand is released then make sure the "SecondHand" Variable is null
  (bind _secondhand (`self.SecondHand`)
    (:`then`
      (if (== _secondhand MotionController)
        (set `self.SecondHand` null)
        (`self.SetActorTickEnabled` false)
        (`self.Shoot`)))
    (:`else`
      ;[1 1 1] If the First Hand is released then drop whatever is in hand (Only If Second Hand Has Been Released)
      (bind _firsthand (`self.FirstHand`)
        (:`then`
          (if (== _firsthand HandMesh)
            (`PrimitiveComponent.SetSimulatePhysics` (`self.StaticMeshComponent`) false)
            (`self.K2_DetachFromActor` "KeepWorld" "KeepWorld" "KeepWorld")
            (set `self.FirstHand` null)
            (set `self.SecondHand` null)))
        (:`else`)))))

(event `self.ReceiveTick`
  (params (DeltaSeconds :type "Float (single-precision)"))
  (bind _returnvalue (- (`self.StringRelativeLocation`) (`SceneComponent.RelativeLocation` (`self.StringCollision`))))
  (bind _returnvalue_2 (`KismetMathLibrary.VSize` _returnvalue))
  ;[1 1 1] Tracks the second hand location when holding string
  (bind _secondhand (`self.SecondHand`)
    (:`then`
      (bind _output_get (set `self.StringRelativeLocation` (`KismetMathLibrary.ProjectVectorOnToVector` (`KismetMathLibrary.InverseTransformLocation` (`self.GetTransform`) (`SceneComponent.K2_GetComponentLocation` _secondhand)) (`KismetMathLibrary.GetForwardVector` (`SceneComponent.RelativeRotation` (`self.StaticMeshComponent`))))))
      (set `self.StringCharge` _returnvalue_2)
      (if (and (not (< (`KismetMathLibrary.Dot_VectorVector` (`KismetMathLibrary.Normal` _returnvalue) (`KismetMathLibrary.GetForwardVector` (`SceneComponent.RelativeRotation` (`self.StaticMeshComponent`)))) 0.0)) (< _returnvalue_2 58.0))
        (`SceneComponent.K2_SetRelativeLocation` (`self.String`) _output_get false false)))
    (:`else`)))

(event `Shoot`
  ;[1 1 1] Make the String snap back to original position when released
  (`TimelineComponent.SetPlayRate` (`self.SnapBack`) (/ 1.0 0.05))
  (bind (_direction _newtrack_0) (`Timeline|SnapBack` :!via `PlayFromStart`)
    (:`Update`
      (`SceneComponent.K2_SetRelativeLocation` (`self.String`) (`KismetMathLibrary.VLerp` (`self.StringRelativeLocation`) (`SceneComponent.RelativeLocation` (`self.StringCollision`)) _newtrack_0) false false)
      ;[1 1 1] If The SnapBack Timeline is at a certain stage and there is an Arrow in the bow, then shoot the arrow
      (if (> _newtrack_0 0.8)
        (bind _arrow (`self.Arrow`)
          (:`then`
            (`self.K2_DetachFromActor` _arrow "KeepWorld" "KeepWorld" "KeepWorld")
            (`/Game/Weapons/Bow/Arrow_BP.Shoot` _arrow (`KismetMathLibrary.MapRangeClamped` (`self.StringCharge`) 0.0 58.0 300.0 3000.0))
            ;[1 1 1] Knockback Of Arrow depends on String Charge
            (`/Game/Weapons/Bow/Arrow_BP.SetArrowPower` _arrow (`KismetMathLibrary.MapRangeClamped` (`self.StringCharge`) 0.0 58.0 50.0 300.0)))
          (:`else`))))))

(fn `UserConstructionScript`)