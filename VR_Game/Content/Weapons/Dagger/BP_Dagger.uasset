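; BP_Dagger is a VR melee weapon that motion controllers pick up, snap to a left or right hand socket, and drop back into physics.
; While held, its AttackBox overlapping an enemy hitbox flags StrongEnemyBP as hit, launches it away and spawns impact effects and sound.
; A C++ Weapon handles damage, with its DamageDealt flag gating hits until a short delay after overlap ends.
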(event `self.ReceiveBeginPlay`
  ;[1 1 1] Find The Player
  (bind _outactors (`GameplayStatics.GetAllActorsOfClass` "/Game/VirtualRealityBP/Blueprints/VRCharacter.VRCharacter_C"))
  (set `Weapon.player` (`|GetArrayItem` _outactors) (`self.Weapon`)))

(event `self.ReceiveTick`
  (params (DeltaSeconds :type "Float (single-precision)")))

(event `/Game/VirtualRealityBP/Blueprints/PickupActorInterface.Pickup`
  (params (MotionController :type "SceneComponent Object Reference") (HandMesh :type "SceneComponent Object Reference") (HandEnum :type "/Game/VirtualRealityBP/Blueprints/WhichHand Enum" :default "NewEnumerator0") (SkeletalMesh :type "SkeletalMeshComponent Object Reference"))
  ;[1 1 1] Set which socket the bow will be attached to
  (switch `/Game/VirtualRealityBP/Blueprints/WhichHand` HandEnum
    (:`NewEnumerator0`
      (set `self.WhichHand` "Dagger_L"))
    (:`NewEnumerator1`
      (set `self.WhichHand` "Dagger_R")))
  (`PrimitiveComponent.SetSimulatePhysics` (`self.StaticMeshComponent`) false)
  (`SceneComponent.K2_AttachToComponent` (`self.K2_GetRootComponent`) SkeletalMesh (`self.WhichHand`) "SnapToTarget" "SnapToTarget" "KeepWorld" false)
  ;[1 1 1] So that the Sword can deal damage only when its been grabbed by player
  (set `Weapon.hasBeenGrabbed` true (`self.Weapon`)))

(event `/Game/VirtualRealityBP/Blueprints/PickupActorInterface.Drop`
  (params (MotionController :type "SceneComponent Object Reference") (HandMesh :type "SceneComponent Object Reference"))
  (`PrimitiveComponent.SetSimulatePhysics` (`self.StaticMeshComponent`) true)
  (`self.K2_DetachFromActor` "KeepWorld" "KeepWorld" "KeepWorld")
  (set `Weapon.hasBeenGrabbed` false (`self.Weapon`)))

(event `Knockback`
  (params (Enemy :type "Character Object Reference"))
  (bind (_returnvalue_x _returnvalue_y) (`KismetMathLibrary.BreakVector` (`KismetMathLibrary.GetDirectionUnitVector` (`SceneComponent.K2_GetComponentLocation` (`self.StaticMeshComponent`)) (`self.K2_GetActorLocation` Enemy))))
  (bind (_returnvalue_x_2 _returnvalue_y_2) (`KismetMathLibrary.BreakVector` (`KismetMathLibrary.Normal` (`KismetMathLibrary.MakeVector` _returnvalue_x _returnvalue_y))))
  ;[1 1 1] Knockback The Player (Parameter will be whatever collided with the Attack Box)
  (`Character.LaunchCharacter` Enemy (* (`KismetMathLibrary.MakeVector` _returnvalue_x_2 _returnvalue_y_2 0.5) (`self.Launch Velocity`)) false false))

(event `self.AttackBox.OnComponentBeginOverlap`
  (params (OverlappedComponent :type "PrimitiveComponent Object Reference") (OtherActor :type "Actor Object Reference") (OtherComp :type "PrimitiveComponent Object Reference") (OtherBodyIndex :type Integer) (bFromSweep :type Boolean) (SweepResult :type "HitResult Structure (by ref)"))
  (bind _weapon (`self.Weapon`))
  ;[1 1 1] If Damage hasnt been dealt yet and the weapon is being grabbed by the player then play the Enemy animation and do the knockback (Damage is done in C++ Script)
  ;;[1 0 0] If Colliding With The Hitbox Of Enemy
  (if (`ActorComponent.ComponentHasTag` OtherComp "EHitbox")
    (if (`Weapon.damageDealt` _weapon)
      _
      (elif (`Weapon.hasBeenGrabbed` _weapon)
        (bind _asstrong_enemy_bp (cast `/Game/Enemies/Strong_Enemy/StrongEnemyBP` OtherActor))
        ;;[1 1 1] This Plays The Enemy Animation
        (set `/Game/Enemies/Strong_Enemy/StrongEnemyBP.BeenHit` true _asstrong_enemy_bp)
        (`self.Knockback` _asstrong_enemy_bp)
        (`NiagaraFunctionLibrary.SpawnSystemAtLocation` "/Game/Particles/NE_WeaponHit_System.NE_WeaponHit_System" (`SceneComponent.K2_GetComponentLocation` (`self.AttackBox`)))
        (`GameplayStatics.PlaySoundAtLocation` "/Game/Sound/WeaponHit.WeaponHit" (`SceneComponent.K2_GetComponentLocation` (`self.StaticMeshComponent`)) (struct) 1.0 1.0 0.0 null null null)))
    (else
      (`KismetSystemLibrary.PrintString` (`KismetSystemLibrary.GetDisplayName` OtherComp)))))

(event `self.AttackBox.OnComponentEndOverlap`
  (params (OverlappedComponent :type "PrimitiveComponent Object Reference") (OtherActor :type "Actor Object Reference") (OtherComp :type "PrimitiveComponent Object Reference") (OtherBodyIndex :type Integer))
  (bind _weapon (`self.Weapon`))
  ;[1 1 1] When the Weapon stops overlapping the enemy and the damageDealt boolean is still true, then after a while set  it to false so the player can attack again
  (if (`Weapon.damageDealt` _weapon)
    (`KismetSystemLibrary.Delay` 0.5)
    (set `Weapon.damageDealt` false _weapon)))

(fn `UserConstructionScript`
  ;[1 1 1] Testing Purposes
  (set `Weapon.CollisionMesh` (`self.AttackBox`) (`self.Weapon`)))