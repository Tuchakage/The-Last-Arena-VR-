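; BP_PickupSword is a sword actor that a motion controller can pick up and drop.
; Pickup disables physics, snaps the root to the supplied component and applies a fixed grip offset to the static mesh.
; Drop re-enables physics and detaches the actor, keeping its world transform.
; The construction script assigns the static mesh as the Weapon's CollisionMesh, a step marked as being for testing.
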(event `/Game/VirtualRealityBP/Blueprints/PickupActorInterface.Pickup`
  (params (AttachTo :type "SceneComponent Object Reference"))
  (`PrimitiveComponent.SetSimulatePhysics` (`self.StaticMeshComponent`) false)
  (`SceneComponent.K2_AttachToComponent` (`self.K2_GetRootComponent`) AttachTo "None" "SnapToTarget" "SnapToTarget" "KeepWorld" false)
  (`SceneComponent.K2_SetRelativeLocationAndRotation` :`self` (`self.StaticMeshComponent`) :`NewLocation` (-3.0 -1.0 30.0)))

(event `/Game/VirtualRealityBP/Blueprints/PickupActorInterface.Drop`
  (`PrimitiveComponent.SetSimulatePhysics` (`self.StaticMeshComponent`) true)
  (`self.K2_DetachFromActor` "KeepWorld" "KeepWorld" "KeepWorld"))

(fn `UserConstructionScript`
  ;[1 1 1] Testing Purposes
  (set `Weapon.CollisionMesh` (`self.StaticMeshComponent`) (`self.Weapon`)))